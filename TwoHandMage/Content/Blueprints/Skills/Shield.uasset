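; Shield skill actor that, when activated off cooldown, becomes visible and enables overlap events on its sphere for a base duration.
; A timer then hides it, disables those overlaps and starts the cooldown, which Tick counts down to zero.
; GetCoolDownFraction exposes the remaining cooldown ratio.
; Damage received is only printed as debug text, with no blocking logic here.
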(event `self.ReceiveAnyDamage`
  (params (Damage :type "Float (single-precision)") (DamageType :type "DamageType Object Reference") (InstigatedBy :type "Controller Object Reference") (DamageCauser :type "Actor Object Reference"))
  (`KismetSystemLibrary.PrintString` (`KismetStringLibrary.Conv_DoubleToString` Damage)))

(event `CallActivate`
  ;[1 1 1] Check cooldown
  (if (== (`self.CooldownLeft`) 0.0)
    (`KismetSystemLibrary.PrintString` "shield")
    (set `PrimitiveComponent.bGenerateOverlapEvents` true (`self.Sphere`))
    (`self.SetActorHiddenInGame` false)
    (bind _returnvalue (`KismetSystemLibrary.K2_SetTimerDelegate` (delegate `DeactivateShield`) (`self.BaseDuration`)))
    (set `self.TimerHandler` _returnvalue)))

(event `DeactivateShield`
  (set `PrimitiveComponent.bGenerateOverlapEvents` false (`self.Sphere`))
  (`self.SetActorHiddenInGame` true)
  (set `self.CooldownLeft` (`self.BaseCooldown`)))

(event `self.ReceiveTick`
  (params (DeltaSeconds :type "Float (single-precision)"))
  (bind _returnvalue (- (`self.CooldownLeft`) DeltaSeconds))
  (set `self.CooldownLeft` (`KismetMathLibrary.SelectFloat` 0.0 _returnvalue (< _returnvalue 0.0))))

(fn `GetCoolDownFraction`
  (returns (CooldownFraction :type "Float (double-precision)"))
  (return (/ (`self.CooldownLeft`) (`self.BaseCooldown`))))

(fn `UserConstructionScript`)