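; Poison cloud skill actor that deals periodic area damage to BaseCharacter pawns within a radius for a limited time.
; SetFields takes duration, radius and damage per second, converts the rate to per-tick damage, draws a debug sphere, then destroys the actor when the duration ends.
; Tick accumulates time and at each TickDelay runs a sphere overlap, applying damage credited to the instigator's controller.
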(event `SetFields`
  (params (Duration :type "Float (double-precision)") (Radius :type "Float (double-precision)") (DamagePerSec :type "Float (double-precision)"))
  (set `self.PosionDuration` Duration)
  (set `self.PoisonRadius` Radius)
  (set `self.DamagePerTick` (/ DamagePerSec (/ 1.0 (`self.TickDelay`))))
  (`KismetSystemLibrary.DrawDebugSphere` (`self.K2_GetActorLocation`) (`self.PoisonRadius`) 12 (struct :`R` 0.411832 :`G` 1.0 :`A` 1.0) (`self.PosionDuration`))
  (`KismetSystemLibrary.Delay` (`self.PosionDuration`))
  (`self.K2_DestroyActor`))

(event `self.ReceiveTick`
  (params (DeltaSeconds :type "Float (single-precision)"))
  (if (>= (`self.CurrentTickTime`) (`self.TickDelay`))
    (set `self.CurrentTickTime` 0.0)
    (`self.Apply Damage to All` (`self.DamagePerTick`))
    (else
      (set `self.CurrentTickTime` (+ (`self.CurrentTickTime`) DeltaSeconds)))))

(fn `Apply Damage to All`
  (params (Damage :type "Float (double-precision)"))
  (bind _outactors (`KismetSystemLibrary.SphereOverlapActors` (`self.K2_GetActorLocation`) (`self.PoisonRadius`) (`|MakeArray` "ObjectTypeQuery3" :!type "EObjectTypeQuery Enum") "/Game/Blueprints/Characters/BaseCharacter.BaseCharacter_C"))
  (for _array_element _outactors
    (`GameplayStatics.ApplyDamage` _array_element Damage (`Pawn.GetController` (`self.GetInstigator`)) self)))

(fn `UserConstructionScript`)