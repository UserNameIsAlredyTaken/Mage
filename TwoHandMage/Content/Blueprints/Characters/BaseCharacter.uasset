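; Base character Blueprint that provides health, damage intake and death.
; Health starts at MaxHealth on BeginPlay, and AnyDamage, unless the character is Invincible or already dead, calls an empty HandleDamage hook before subtracting the clamped damage.
; At zero health Die destroys the actor, and GetCurrentHealthFraction exposes health as a ratio of the maximum.
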(event `self.ReceiveAnyDamage`
  (params (Damage :type "Float (single-precision)") (DamageType :type "DamageType Object Reference") (InstigatedBy :type "Controller Object Reference") (DamageCauser :type "Actor Object Reference"))
  (if (not (`self.Invincible`))
    (set `self.Damage` Damage)
    ;[1 1 1] Check if already dead
    (if (> (`self.CurrentHealth`) 0.0)
      (`self.HandleDamage` (`self.Damage`))
      (bind _output_get (set `self.CurrentHealth` (`KismetMathLibrary.FClamp` (- (`self.CurrentHealth`) (`self.Damage`)) 0.0 (`self.MaxHealth`))))
      (if (<= _output_get 0.0)
        (`self.Die`)))))

(event `self.ReceiveBeginPlay`
  (set `self.CurrentHealth` (`self.MaxHealth`)))

(fn `Die`
  (`self.K2_DestroyActor`))

(fn `GetCurrentHealthFraction`
  (returns (Fraction :type "Float (double-precision)"))
  (return (/ (`self.CurrentHealth`) (`self.MaxHealth`))))

(fn `HandleDamage`
  (params (GottenDmg :type "Float (double-precision)")))

(fn `UserConstructionScript`)