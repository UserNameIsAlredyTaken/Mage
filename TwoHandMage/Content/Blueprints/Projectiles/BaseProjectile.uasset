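; Base projectile Blueprint that routes collision events from its CollisionComponent into a shared HandleCollision function, which is empty here.
; Overlaps ignore the owner and actors tagged Projectile, then report with Hit false, while blocking hits report unfiltered with Hit true.
; An unconnected chain would briefly ignore world and physics-body channels after spawn, but it never runs.
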(event `self.ReceiveBeginPlay`)

(event `self.CollisionComponent.OnComponentBeginOverlap`
  (params (OverlappedComponent :type "PrimitiveComponent Object Reference") (OtherActor :type "Actor Object Reference") (OtherComp :type "PrimitiveComponent Object Reference") (OtherBodyIndex :type Integer) (bFromSweep :type Boolean) (SweepResult :type "HitResult Structure (by ref)"))
  (if (not (or (== OtherActor (`self.GetOwner`)) (`self.ActorHasTag` OtherActor "Projectile")))
    (`self.HandleCollision` OtherActor)))

(event `self.CollisionComponent.OnComponentHit`
  (params (HitComponent :type "PrimitiveComponent Object Reference") (OtherActor :type "Actor Object Reference") (OtherComp :type "PrimitiveComponent Object Reference") (NormalImpulse :type "Vector Structure") (Hit :type "HitResult Structure (by ref)"))
  (`self.HandleCollision` OtherActor true))

(fn `HandleCollision`
  (params (OtherActor :type "Actor Object Reference") (bHit :type Boolean)))

(fn `UserConstructionScript`)